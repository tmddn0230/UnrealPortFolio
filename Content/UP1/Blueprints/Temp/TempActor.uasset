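; TempActor is a test actor that moves its static mesh in response to spoken voice commands.
; On BeginPlay it binds TriggerSpeech to the SpeechRecognitionSubsystem's words-spoken event, and on EndPlay it shuts that subsystem down.
; Each recognized phrase is printed and string-matched: several commands share one upward impulse, "move" applies a stronger one, and "get" only prints.
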(event `self.ReceiveBeginPlay`
  (add `SpeechRecognitionSubsystem.OnWordsSpoken` (subsystem `SpeechRecognitionSubsystem`) (delegate `TriggerSpeech`)))

(event `TriggerSpeech`
  (params (Text :type "RecognisedPhrases Structure"))
  (bind _staticmesh (`self.StaticMesh`))
  (for _array_element (`.phrases` (break `RecognisedPhrases` Text))
    (`KismetSystemLibrary.PrintString` _array_element)
    (if (== _array_element "turn off gravity")
      (`PrimitiveComponent.AddImpulse` _staticmesh (0.0 0.0 10000.0) "None" false :!label _label)
      (elif (== _array_element "go away")
        (goto _label)
        (elif (== _array_element "gone")
          (goto _label)
          (elif (== _array_element "get")
            (`KismetSystemLibrary.PrintString` "Get")
            (elif (== _array_element "move")
              (`PrimitiveComponent.AddImpulse` _staticmesh (0.0 0.0 20000.0) "None" false))))))))

(event `self.ReceiveEndPlay`
  (params (EndPlayReason :type "EEndPlayReason Enum" :default "Destroyed"))
  (`SpeechRecognitionSubsystem.Shutdown` (subsystem `SpeechRecognitionSubsystem`)))

(fn `UserConstructionScript`)