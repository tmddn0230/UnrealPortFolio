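; Push-to-talk speech-to-text actor that records audio and prints an OpenAI transcription of it.
; On BeginPlay it enables input and loads the API key from environment variables, but only if an audio capture device exists.
; Holding Q records a submix to a WAV at a hard-coded local path.
; The file-done event sends it after a short delay, with a DoOnce that resets only on success, so a failure blocks later transcriptions.
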(event `self.ReceiveBeginPlay`
  (bind _outdevices (`MediaBlueprintFunctionLibrary.EnumerateAudioCaptureDevices` -1))
  (bind _output_get (set `self.Enabled` (> (`KismetArrayLibrary.Array_Length` _outdevices) 0)))
  (if _output_get
    (`self.EnableInput` (`GameplayStatics.GetPlayerController` 0))
    (`OpenAIUtils.setUseOpenAIApiKeyFromEnvironmentVars` true)))

(event `Key|Q`
  (params (Key :type "Key Structure"))
  (bind _submix_to_record (`self.Submix to Record`))
  (:`Pressed`
    (`AudioMixerBlueprintLibrary.StartRecordingOutput` 0.0 _submix_to_record))
  (:`Released`
    (`AudioMixerBlueprintLibrary.StopRecordingOutput` "WavFile" (`self.FileName`) "C:\\Users\\inter\\Documents\\GitHub\\UnrealPortFolio" _submix_to_record null)))

(event `self.Submix to Record.OnSubmixRecordedFileDone`
  (params (ResultingSoundWave :type "SoundWave Object Reference"))
  (`/Engine/EditorBlueprintResources/StandardMacros.DoOnce` false :!label _label
    (:`Completed`
      (`KismetSystemLibrary.Delay` 0.2)
      (bind (_transcription _errormessage _success) (`OpenAICallTranscriptions.OpenAICallTranscriptions` (`self.FileName`))
        (:`Finished`
          (if _success
            (`KismetSystemLibrary.PrintString` _transcription)
            (goto _label :!via `Reset`)
            (else
              (`KismetSystemLibrary.PrintString` _errormessage))))))))

(fn `UserConstructionScript`)